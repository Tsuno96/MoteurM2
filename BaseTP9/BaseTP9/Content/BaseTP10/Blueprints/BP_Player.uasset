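; Player Blueprint that provides a mouse-cursor camera view for placing BP_Al and BP_Muffin actors in the level.
; The MoveForward axis zooms the camera along its line to the root, stepping proportionally to the remaining distance.
; Spawn inputs trace from the deprojected cursor and spawn scaled actors only on BP_SpawnArea hits.
; Input names are mismatched: SpawnMuffin spawns BP_Al, while SpawnBuffin spawns BP_Muffin.
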(event EventBeginPlay
  (bind _returnvalue (Game|GetPlayerController 0))
  (Variables|/Script/Engine.PlayerController|SetbShowMouseCursor _returnvalue true)
  (Input|EnableInput _returnvalue))

(event Input|ActionEvents|InputActionSpawnBuffin
  (params (Key :type Key%20Structure :default "None"))
  (bind _returnvalue (Game|GetPlayerController 0))
  (bind (_worldlocation _worlddirection) (Game|Player|ConvertMouseLocationToWorldSpace _returnvalue))
  (:Pressed
    (bind _outhit (Collision|LineTraceByChannel _worldlocation (+ _worldlocation (* _worlddirection (Variables|Default|GetTraceDistance))) "TraceTypeQuery1" false 0 "None"))
    (Utilities|Casting|CastToBP_SpawnArea (.HitActor (Collision|BreakHitResult _outhit)))
    (Game|SpawnActorfromClass "/Game/BaseTP10/Characters/Muffin/Blueprints/BP_Muffin.BP_Muffin_C" (Math|Transform|MakeTransform (.Location (Collision|BreakHitResult _outhit)) "0, 0, 0" "2.000000,2.000000,2.000000") "AdjustIfPossibleButAlwaysSpawn" 0 0)))

(event Input|ActionEvents|InputActionSpawnMuffin
  (params (Key :type Key%20Structure :default "None"))
  (bind _returnvalue (Game|GetPlayerController 0))
  (bind (_worldlocation _worlddirection) (Game|Player|ConvertMouseLocationToWorldSpace _returnvalue))
  (:Pressed
    (bind _outhit (Collision|LineTraceByChannel _worldlocation (+ _worldlocation (* _worlddirection (Variables|Default|GetTraceDistance))) "TraceTypeQuery1" false 0 "None"))
    (Utilities|Casting|CastToBP_SpawnArea (.HitActor (Collision|BreakHitResult _outhit)))
    (Game|SpawnActorfromClass "/Game/BaseTP10/Characters/AlcaponeVoxels/BluePrints/BP_Al.BP_Al_C" (Math|Transform|MakeTransform (.Location (Collision|BreakHitResult _outhit)) "0, 0, 0" "8.000000,8.000000,8.000000") "AdjustIfPossibleButAlwaysSpawn" 0 0)))

(event Input|AxisEvents|InputAxisMoveForward
  (params (AxisValue :type Float%20%28single-precision%29))
  (bind _camera (Variables|Default|GetCamera))
  (bind _defaultsceneroot (Variables|Default|GetDefaultSceneRoot))
  (bind _returnvalue (Transformation|GetWorldLocation _camera))
  (bind _returnvalue_2 (Transformation|GetWorldLocation _defaultsceneroot))
  (bind _returnvalue_3 (- _returnvalue_2 _returnvalue))
  (Transformation|SetWorldLocation (Variables|Default|GetCamera) (+ _returnvalue (* (Math|Vector|Normalize _returnvalue_3) (* (* AxisValue 0.1) (Math|Vector|VectorLength _returnvalue_3)))) false false))

(fn ConstructionScript)